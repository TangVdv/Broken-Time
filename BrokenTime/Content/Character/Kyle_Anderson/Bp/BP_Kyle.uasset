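; BP_Kyle is the player character Blueprint, handling camera look, movement and sprinting with stamina.
; Look input updates an aim Pitch and, while standing still, sets TurnLeft/TurnRight flags, while movement follows control yaw.
; Sprint switches walk speed and starts a looping GestionEndurance timer that drains Endurance while running, drops to walk speed when empty, and pauses once regenerated to max.
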(event `InputAxis|LookUp`
  (params (AxisValue :type "Float (single-precision)"))
  (bind (_returnvalue_roll _returnvalue_pitch) (`KismetMathLibrary.BreakRotator` (`KismetMathLibrary.NormalizedDeltaRotator` (`self.GetControlRotation`) (`self.K2_GetActorRotation`))))
  (`self.AddControllerPitchInput` AxisValue)
  (bind _output_get (set `self.Pitch` _returnvalue_pitch))
  (set `self.Pitch` (+ _output_get 1.0)))

(event `InputAxis|Turn`
  (params (AxisValue :type "Float (single-precision)"))
  ;[1 1 1] Caméra
  (`|ExecutionSequence`
    (:`then_0`
      (`self.AddControllerYawInput` AxisValue))
    (:`then_1`
      (if (== (`self.GetVelocity`) (0.0 0.0 0.0) :`ErrorTolerance` 0.01)
        (`|ExecutionSequence`
          (:`then_0`
            (if (> AxisValue 0.3)
              (set `self.TurnRight ?` true)
              (set `self.TurnLeft?` false)
              (else
                (set `self.TurnRight ?` false))))
          (:`then_1`
            (if (< AxisValue -0.3)
              (set `self.TurnLeft?` true)
              (else
                (set `self.TurnLeft?` false)))))
        (else
          (set `self.TurnLeft?` false)
          (set `self.TurnRight ?` false))))
    (:`then_2`
      (set `self.TurnRight ?` (`self.TurnRight ?`))
      (set `self.TurnLeft?` (`self.TurnLeft?`)))))

(event `InputAxis|MoveForward`
  (params (AxisValue :type "Float (single-precision)"))
  ;[1 1 1] Déplacement
  (`self.AddMovementInput` (`KismetMathLibrary.GetForwardVector` (`KismetMathLibrary.MakeRotator` 0.0 0.0 (.yaw (`self.GetControlRotation`)))) AxisValue))

(event `InputAxis|MoveRight`
  (params (AxisValue :type "Float (single-precision)"))
  ;[1 1 1] Déplacement
  (`self.AddMovementInput` (`KismetMathLibrary.GetRightVector` (`KismetMathLibrary.MakeRotator` 0.0 0.0 (.yaw (`self.GetControlRotation`)))) AxisValue))

(event `InputAction|Sprint`
  (params (Key :type "Key Structure"))
  (bind _charactermovement (`self.CharacterMovement`))
  ;[1 1 1] Sprint/Stamina
  (:`Pressed`
    (set `CharacterMovementComponent.MaxWalkSpeed` 600.0 _charactermovement)
    (set `self.IsRunning?` (== (`CharacterMovementComponent.MaxWalkSpeed` (`self.CharacterMovement`)) 600.0) :!label _label)
    (bind _returnvalue (`KismetSystemLibrary.K2_SetTimer` null "GestionEndurance" 0.01 true))
    (set `self.TimerEndurance` _returnvalue))
  (:`Released`
    (set `CharacterMovementComponent.MaxWalkSpeed` 300.0 _charactermovement)
    (goto _label)))

(event `self.ReceiveBeginPlay`)

(fn `GestionEndurance`
  (if (and (`MovementComponent.IsExceedingMaxSpeed` (`self.CharacterMovement`) 100.0) (`self.IsRunning?`))
    (if (> (`self.Endurance`) 0.0)
      (set `self.Endurance` (- (`self.Endurance`) 0.1))
      (else
        (set `CharacterMovementComponent.MaxWalkSpeed` 300.0 (`self.CharacterMovement`))))
    (elif (< (`self.Endurance`) (`self.EnduranceMax`))
      (set `self.Endurance` (+ (`self.Endurance`) 0.05))
      (else
        (`KismetSystemLibrary.K2_PauseTimerHandle` (`self.TimerEndurance`))))))

(fn `UserConstructionScript`)